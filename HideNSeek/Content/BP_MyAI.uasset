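; BP_MyAI is an AI agent in a tag-style game, carrying an IsIt flag that marks whether it is "it".
; On BeginPlay it copies IsIt into its BP_MyAIController's blackboard.
; When it is "it" and overlaps a BP_MyAI2, it sets that agent's IsIt and clears its own.
; The handoff changes only the actor variables, leaving the blackboard value untouched.
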(event EventBeginPlay
  (bind _asbp_my_aicontroller (Utilities|Casting|CastToBP_MyAIController (AI|GetAIController self)))
  (AI|Components|Blackboard|SetValueasBool (AI|GetBlackboard _asbp_my_aicontroller) (Utilities|Name|MakeLiteralName "IsIt") (Variables|Default|GetIsIt)))

(event Collision|EventActorBeginOverlap
  (params (OtherActor :type Actor%20Object%20Reference))
  (if (Variables|Default|GetIsIt)
    (bind _asbp_my_ai2 (Utilities|Casting|CastToBP_MyAI2 OtherActor))
    (Variables|/Game/BP_MyAI2.BP_MyAI2_C|SetIsIt _asbp_my_ai2 true)
    (Variables|Default|SetIsIt false)))

(event EventTick
  (params (DeltaSeconds :type Float%20%28single-precision%29)))

(fn ConstructionScript)